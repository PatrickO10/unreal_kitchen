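; BP_Plate is a plate actor that can be picked up and dropped, apparently by the player in VR.
; PickUp turns off physics on the plate mesh, stores the target and attaches the root component to it, keeping world transform.
; DropOff restores physics, detaches, clears the target and gives the plate a small upward impulse.
; BeginPlay caches the player's MyVRPawn, which the graph does not otherwise use.
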(event EventBeginPlay
  ;[1 1 1] Reference to MyVRPawn
  (bind _asmy_vrpawn (Utilities|Casting|CastToMyVRPawn (Game|Player|GetPlayerPawn 0)))
  (Variables|Default|SetMyVRPawn _asmy_vrpawn))

(event Collision|EventActorBeginOverlap
  (params (OtherActor :type Actor%20Object%20Reference)))

(event EventTick
  (params (DeltaSeconds :type Float%20%28single-precision%29)))

(event EventPickUp
  (params (ActorToAttachTo :type Scene%20Component%20Object%20Reference))
  (Variables|Default|SetTarget ActorToAttachTo)
  (Physics|SetSimulatePhysics (Variables|Default|Getplate) false)
  (Transformation|AttachComponentToComponent (VehicleSound|GetRootComponent) ActorToAttachTo "None" "KeepWorld" "KeepWorld" "KeepWorld" true))

(event EventDropOff
  (Physics|SetSimulatePhysics (Variables|Default|Getplate) true)
  (Transformation|DetachFromActor "KeepWorld" "KeepWorld" "KeepWorld")
  (Variables|Default|SetTarget 0)
  (Physics|AddImpulse (Variables|Default|Getplate) "0, 0,50.000000" "None" false))

(fn ConstructionScript)