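; Sink actor for a VR game that washes carried plates and awards points for them.
; When a bp_plate flagged as picked overlaps its Box, it plays a water sound at the sink.
; After a short delay it plays a pop sound at the plate, destroys it and adds its Score value through MyVRGameMode.
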(event OnComponentBeginOverlap(Box)
  (params (OverlappedComponent :type Primitive%20Component%20Object%20Reference) (OtherActor :type Actor%20Object%20Reference) (OtherComp :type Primitive%20Component%20Object%20Reference) (OtherBodyIndex :type Integer) (bFromSweep :type Boolean) (SweepResult :type Hit%20Result%20Structure%20%28by%20ref%29))
  ;[1 1 1] When BeginOverlap play a washing sound
  (bind _asbp_plate (Utilities|Casting|CastTobp_plate OtherActor))
  (if (and (== OtherActor _asbp_plate) (Variables|/Game/Assets/blueprints/bp_plate.bp_plate_C|GetObjectPicked _asbp_plate))
    (Audio|PlaySoundatLocation "/Game/Assets/audio/VR_objectRotateLoop_water_Cue.VR_objectRotateLoop_water_Cue" (Transformation|GetActorLocation))
    ;[1 1 1] Cast to bp_plate and destroy actor when washing is complete
    (bind _asbp_plate_2 (Utilities|Casting|CastTobp_plate OtherActor))
    (Utilities|FlowControl|Delay 1.0)
    (Audio|PlaySoundatLocation "/Game/Assets/audio/a_balloonPop_Cue.a_balloonPop_Cue" (Transformation|GetActorLocation _asbp_plate_2))
    (Actor|DestroyActor _asbp_plate_2)
    ;[1 1 1] Add point if plate is successfully destroyed
    (bind _asmy_vrgame_mode (Utilities|Casting|CastToMyVRGameMode (Game|GetGameMode)))
    (Default|AddScore _asmy_vrgame_mode (Variables|Default|GetScore))))

(event EventBeginPlay)

(event Collision|EventActorBeginOverlap
  (params (OtherActor :type Actor%20Object%20Reference)))

(event EventTick
  (params (DeltaSeconds :type Float%20%28single-precision%29)))

(fn ConstructionScript)