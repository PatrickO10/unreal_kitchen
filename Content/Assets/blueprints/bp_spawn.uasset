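; Spawner actor that creates Bp_plate actors at the transforms of randomly chosen Bp_targets actors in the level.
; BeginPlay, or the player pawn entering CollisionStartBox, gathers the targets and plays the Waves timeline.
; Each Wave 1 event on that timeline spawns one plate at a random target, ignoring collisions.
; The SpawnPlates function is an empty stub.
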(event OnComponentBeginOverlap(CollisionStartBox)
  (params (OverlappedComponent :type Primitive%20Component%20Object%20Reference) (OtherActor :type Actor%20Object%20Reference) (OtherComp :type Primitive%20Component%20Object%20Reference) (OtherBodyIndex :type Integer) (bFromSweep :type Boolean) (SweepResult :type Hit%20Result%20Structure%20%28by%20ref%29))
  ;[1 1 1] If overlap is pawn then spawn plates
  (if (== OtherActor (Game|Player|GetPlayerPawn 0))
    (bind _outactors (Actor|GetAllActorsOfClass "/Game/Assets/blueprints/bp_targets.bp_targets_C"))
    (Timeline|Waves Play
      (:Wave_1
        (Game|SpawnActorfromClass "/Game/Assets/blueprints/bp_plate.bp_plate_C" (Transformation|GetActorTransform (Utilities|Array|Get(acopy) _outactors (Math|Random|RandomIntegerinRange 0 (- (Utilities|Array|Length _outactors) 1)))) "AlwaysSpawn" 0 0)))))

(event EventBeginPlay
  (bind _outactors (Actor|GetAllActorsOfClass "/Game/Assets/blueprints/bp_targets.bp_targets_C"))
  (Timeline|Waves Play
    (:Wave_1
      (Game|SpawnActorfromClass "/Game/Assets/blueprints/bp_plate.bp_plate_C" (Transformation|GetActorTransform (Utilities|Array|Get(acopy) _outactors (Math|Random|RandomIntegerinRange 0 (- (Utilities|Array|Length _outactors) 1)))) "AlwaysSpawn" 0 0))))

(event Collision|EventActorBeginOverlap
  (params (OtherActor :type Actor%20Object%20Reference)))

(event EventTick
  (params (DeltaSeconds :type Float%20%28single-precision%29)))

(fn ConstructionScript)

(fn SpawnPlates)